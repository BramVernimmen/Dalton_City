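; GM_Game is the match game mode that tracks joining players and advances the match state once the lobby is full.
; On BeginPlay it reads the maximum player count from the session's "Players" extra setting.
; PostLogin counts joins, sets the new match state on GS_Game when the count hits the maximum, and sends any later joiner back to the main menu through their PC_Game.
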(event EventPostLogin
  (params (NewPlayer :type Player%20Controller%20Object%20Reference))
  (if (< (Variables|Default|GetPlayerCount) (Variables|Default|GetMaxPlayers))
    (bind _result (Math|Integer|IncrementInt (Variables|Default|GetPlayerCount))
      (:%20%20
        (if (== _result (Variables|Default|GetMaxPlayers))
          (CallFunction|ChangeMatchState "NewEnumerator1"))))
    (else
      ;[1 1 1] If we have all players, kick others to main menu
      (bind _aspc_game (Utilities|Casting|CastToPC_Game NewPlayer))
      (Default|SendBacktoMainMenu _aspc_game))))

(event EventBeginPlay
  ;[1 1 1] Set the max amount of players
  (bind _extrasettings (Class|AdvancedSessionsLibrary|GetSessionSettings)
    (:OnSuccess
      (bind _settingvalue (Class|AdvancedSessionsLibrary|GetSessionPropertyInt _extrasettings "Players")
        (:Found
          (Variables|Default|SetMaxPlayers _settingvalue))))))

(fn ConstructionScript)

(fn ChangeMatchState
  (params (New%20Match%20State :type ENUM_MatchState%20Enum :default "NewEnumerator0"))
  (bind _asgs_game (Utilities|Casting|CastToGS_Game (Game|GetGameState)))
  (Variables|/Game/Blueprints/Game/GS_Game.GS_Game_C|SetCurrent%20Match%20State _asgs_game New%20Match%20State))
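; Player controller for a multiplayer tile board game, handling the camera, HUD, player name, money and pawn.
; In pre-game, left-clicking a Ranch tile spawns a pawn via the server, claimed after a delay by searching for unowned pawns.
; Turns move a fixed three spaces, recursively lerping tile to tile on a timeline before registering the final tile with GS_Game.
; Name and money OnReps trigger GS_Game updates for the HUD.
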(event Custom|Send%20Back%20To%20Main%20Menu
  ;[1 1 1] If this player shouldn't be allowed to join the game, open main menu
  (Game|OpenLevel(byName) "MainMenu_Level"))

(event Custom|Update%20Player%20Money
  (bind _asgs_game (Utilities|Casting|CastToGS_Game (Game|GetGameState)))
  (Default|ServerUpdatePlayerMoney _asgs_game))

(event Custom|Do%20Turn
  (Utilities|FlowControl|Delay 1.0)
  (CallFunction|MovePawn 3))

(event Custom|Local%20Set%20New%20Player
  (params (Player :type Player%20State%20Object%20Reference))
  (CallFunction|ServerSetNewPlayer Player))

(event Custom|Server%20Set%20New%20Player
  (params (Player :type Player%20State%20Object%20Reference))
  (bind _asgs_game (Utilities|Casting|CastToGS_Game (Game|GetGameState)))
  (Default|SetNewCurrentPlayer _asgs_game Player))

(event Custom|Call%20Pick%20Player
  (bind _asgs_game (Utilities|Casting|CastToGS_Game (Game|GetGameState)))
  (bind _player (Default|PickNextPlayer _asgs_game))
  (CallFunction|LocalSetNewPlayer _player))

(event Custom|Local%20Set%20Display%20Pawn
  (params (Pawn :type BP%20Pawn%20Object%20Reference))
  (Utilities|FlowControl|Delay 0.25)
  (bind _outactors (Actor|GetAllActorsOfClass "/Game/Blueprints/Game/Logic/BP_Pawn.BP_Pawn_C"))
  (for _array_element _outactors
    (if (not (Variables|/Game/Blueprints/Game/Logic/BP_Pawn.BP_Pawn_C|GetHasOwner _array_element))
      (if (== (Variables|Default|GetDisplayPawn) 0)
        (bind _output_get (Variables|Default|SetDisplayPawn _array_element))
        (CallFunction|ServerSetPawnHasOwner _output_get)))))

(event Custom|Server%20Set%20Pawn%20Has%20Owner
  (params (Pawn :type BP%20Pawn%20Object%20Reference))
  (Variables|/Game/Blueprints/Game/Logic/BP_Pawn.BP_Pawn_C|SetHasOwner Pawn true))

(event Custom|Server%20Set%20Pawn%20Actor%20Location
  (params (Pawn :type BP%20Pawn%20Object%20Reference) (New%20Location :type Vector))
  (Transformation|SetActorLocation Pawn New%20Location false false))

(event Custom|Server%20Assign%20Player%20To%20Tile
  (params (Player :type PC%20Game%20Object%20Reference) (Tile :type BP%20Tile%20Object%20Reference))
  (bind _asgs_game (Utilities|Casting|CastToGS_Game (Game|GetGameState)))
  (Default|AssignPlayertoTile _asgs_game Player Tile))

(event Custom|Change%20Money
  (params (New%20Amount :type Integer))
  (Variables|Default|SetCurrentMoney New%20Amount))

(event Custom|Notify%20Game%20State%20Of%20Tile
  (params (Clicked%20Tile :type BP%20Tile%20Object%20Reference))
  (bind _asgs_game (Utilities|Casting|CastToGS_Game (Game|GetGameState)))
  (Default|AssignPlayertoTile _asgs_game self Clicked%20Tile))

(event Custom|Server%20Spawn%20Pawn
  (params (Transform :type Transform) (NewParam :type PC%20Game%20Object%20Reference))
  (bind _returnvalue (Game|SpawnActorfromClass "/Game/Blueprints/Game/Logic/BP_Pawn.BP_Pawn_C" Transform "Undefined" "MultiplyWithRoot" 0 0))
  (CallFunction|LocalSetDisplayPawn _returnvalue))

(event Custom|Move%20Pawn
  (params (Amount%20Of%20Spaces :type Integer))
  (bind _asgs_game (Utilities|Casting|CastToGS_Game (Game|GetGameState)))
  (bind _start_tile (Default|FindTileOfPlayer _asgs_game self))
  (Variables|Movement|SetCached%20Tile _start_tile)
  (if (> Amount%20Of%20Spaces 0)
    (CallFunction|MoveLogic Amount%20Of%20Spaces _asgs_game)))

(event Custom|Add%20Money
  (params (Amount%20To%20Add :type Integer))
  (Variables|Default|SetCurrentMoney (+ Amount%20To%20Add (Variables|Default|GetCurrentMoney))))

(event Custom|Move%20Logic
  (params (Amount%20Of%20Spaces :type Integer) (Game%20State :type GS%20Game%20Object%20Reference))
  (if (> Amount%20Of%20Spaces 0)
    (bind _cached_tile (Variables|Movement|GetCached%20Tile)
      (:then
        (bind _next_tile (Default|GetNextTile Game%20State _cached_tile))
        (Variables|Movement|SetCached%20Tile _next_tile)
        (Variables|Default|GetDisplayPawn
          (:then
            (bind _alpha (Timeline|MovePawn PlayFromStart)
              (:Update
                (bind _displaypawn (Variables|Default|GetDisplayPawn)
                  (:then
                    (bind _cached_tile_2 (Variables|Movement|GetCached%20Tile)
                      (:then
                        (CallFunction|ServerSetPawnActorLocation (Variables|Default|GetDisplayPawn) (Math|Vector|Lerp(Vector) (Transformation|GetActorLocation _displaypawn) (Transformation|GetActorLocation _cached_tile_2) _alpha)))
                      (:else)))
                  (:else)))
              (:Finished
                (CallFunction|MoveLogic (- Amount%20Of%20Spaces 1) Game%20State))))
          (:else
            (CallFunction|CallPickPlayer))))
      (:else))
    (else
      (CallFunction|ServerAssignPlayertoTile self (Variables|Movement|GetCached%20Tile)))))

(event Custom|Remove%20Money
  (params (Amount%20To%20Remove :type Integer))
  (Variables|Default|SetCurrentMoney (- (Variables|Default|GetCurrentMoney) Amount%20To%20Remove)))

(event Custom|Local%20Create%20Start%20Text
  (bind _returnvalue (UserInterface|CreateWidget "/Game/Widgets/Game_Widgets/WB_StartText.WB_StartText_C" self))
  (Variables|Default|SetStartText _returnvalue)
  (UserInterface|Viewport|AddtoViewport (Variables|Default|GetStartText) 0))

(event EventBeginPlay
  (if (Pawn|IsLocalController)
    (Utilities|FlowControl|Sequence
      (:then_0
        ;[1 1 1] Set the game camera as active
        (bind _outactors (Actor|GetAllActorsOfClass "/Script/Engine.CameraActor"))
        (Game|Player|SetViewTargetwithBlend (Utilities|Array|Get(acopy) _outactors) 0.0 "VTBlend_Linear" 0.0 false)
        (Variables|Default|SetbShowMouseCursor true))
      (:then_1
        (CallFunction|CreateGameHud))
      (:then_2
        (CallFunction|InitializeName))
      (:then_3
        (CallFunction|ChangeMoney 5000)))))

(event Input|MouseEvents|LeftMouseButton
  (params (Key :type Key%20Structure :default "None"))
  (:Pressed
    (bind _asgs_game (Utilities|Casting|CastToGS_Game (Game|GetGameState)))
    (switch Utilities|FlowControl|Switch|SwitchonENUM_MatchState (Variables|/Game/Blueprints/Game/GS_Game.GS_Game_C|GetCurrent%20Match%20State _asgs_game)
      (:NewEnumerator1
        (bind _pawnspawned (CallFunction|SpawnPawn))
        (if _pawnspawned
          (bind _starttext (Variables|Default|GetStartText)
            (:then
              (Widget|RemovefromParent _starttext))
            (:else)))))))

(event Input|MouseEvents|RightMouseButton
  (params (Key :type Key%20Structure :default "None"))
  (bind _returnvalue (Game|GetPlayerController 0))
  (bind _hitresult (Game|Player|GetHitResultUnderCursorbyChannel _returnvalue "TraceTypeQuery1" true))
  (bind (_bblockinghit _binitialoverlap _time _distance _location _impactpoint _normal _impactnormal _physmat _hitactor) (Collision|BreakHitResult _hitresult))
  (:Pressed
    (if _bblockinghit
      (Utilities|Casting|CastToBP_Tile _hitactor))))

(event Custom|Update%20Player%20Names
  (bind _asgs_game (Utilities|Casting|CastToGS_Game (Game|GetGameState)))
  (Default|ServerUpdatePlayerNames _asgs_game))

(event Custom|Local%20Update%20Game%20HUD
  (params (PlayerNames :type Array%20of%20Strings) (PlayerMoney :type Array%20of%20Integers))
  (bind _game_hud (Variables|Default|GetGame%20Hud)
    (:then
      (Default|SetPlayerNames _game_hud PlayerNames)
      (Default|SetPlayerMoney _game_hud PlayerMoney))
    (:else)))

(event Custom|ServerSetPlayerName
  (params (Player%20Name :type String))
  ;[1 1 1] After getting it locally, set it as the server
  (Variables|Default|SetPlayerName Player%20Name))

(event Custom|InitializeName
  ;[1 1 1] We need to correctly get our Player Name, which is stored in the Game Instance
  (CallFunction|LocalInitializePlayerName))

(event Custom|Local%20Initialize%20Player%20Name
  ;[1 1 1] First get it locally, otherwise you will use the GameInstance of the Server
  (CallFunction|ServerSetPlayerName (CallFunction|GetPlayerName)))

(fn ConstructionScript)

(fn CreateGameHud
  (bind _returnvalue (UserInterface|CreateWidget "/Game/Widgets/Game_Widgets/WB_GameHud.WB_GameHud_C" self))
  (bind _output_get (Variables|Default|SetGame%20Hud _returnvalue))
  (UserInterface|Viewport|AddtoViewport _output_get 0))

(fn OnRepPlayerName
  (if (Pawn|IsLocalController)
    (CallFunction|UpdatePlayerNames)))

(fn GetPlayerName
  (bind _asbp_game_instance (Utilities|Casting|CastToBP_GameInstance (Game|GetGameInstance)))
  (return (Variables|/Game/Blueprints/BP_GameInstance.BP_GameInstance_C|GetPlayerName _asbp_game_instance)))

(fn OnRepCurrentMoney
  (if (Pawn|IsLocalController)
    (CallFunction|UpdatePlayerMoney)))

(fn SpawnPawn
  (bind _returnvalue (Game|GetPlayerController 0))
  (bind _hitresult (Game|Player|GetHitResultUnderCursorbyChannel _returnvalue "TraceTypeQuery1" true))
  (bind (_bblockinghit _binitialoverlap _time _distance _location _impactpoint _normal _impactnormal _physmat _hitactor) (Collision|BreakHitResult _hitresult))
  ;[1 1 1] Only spawn if there is nothing yet
  (if (== (Variables|Default|GetDisplayPawn) 0)
    ;[1 1 1] Check if the player clicked on a tile
    (if _bblockinghit
      (bind _asbp_tile (Utilities|Casting|CastToBP_Tile _hitactor))
      ;[1 1 1] Players should only be allowed to spawn on "Ranch" type tiles
      (if (> (Utilities|Array|Length (Actor|GetComponentsByClass _asbp_tile "/Game/Blueprints/Game/Logic/TileTypes/BP_Ranch.BP_Ranch_C")) 0)
        ;[1 1 1] Spawn the Pawn
        (CallFunction|ServerSpawnPawn (Transformation|GetActorTransform _asbp_tile) self)
        (CallFunction|NotifyGameStateOfTile _asbp_tile)
        (return true)
        (else
          _))))
  (return false))
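; BP_Tile is a game tile that tracks the players on it and triggers its effects when someone lands.
; On BeginPlay it caches its BP_BaseType components, so effects are composed as components on the tile.
; AddPlayer updates the Players list and calls OnPlayerAdded, which executes every cached component only while the GS_Game match state is In Game.
; RemovePlayer only updates the list.
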(event Custom|Add%20Player
  (params (Player%20To%20Add :type PC%20Game%20Object%20Reference))
  ;[1 1 1] Adding a Player here will trigger the notify
  (Utilities|Array|Add (Variables|Default|GetPlayers) Player%20To%20Add)
  (CallFunction|OnPlayerAdded))

(event Custom|Remove%20Player
  (params (Player%20To%20Remove :type PC%20Game%20Object%20Reference))
  (Utilities|Array|RemoveItem (Variables|Default|GetPlayers) Player%20To%20Remove))

(event EventBeginPlay
  (Variables|Default|SetGameComponents (Actor|GetComponentsByClass "/Game/Blueprints/Game/Logic/TileTypes/BP_BaseType.BP_BaseType_C")))

(fn ConstructionScript)

(fn OnPlayerAdded
  ;[1 1 1] Only when InGame, trigger effects
  (bind _asgs_game (Utilities|Casting|CastToGS_Game (Game|GetGameState)))
  (switch Utilities|FlowControl|Switch|SwitchonENUM_MatchState (Variables|/Game/Blueprints/Game/GS_Game.GS_Game_C|GetCurrent%20Match%20State _asgs_game)
    (:NewEnumerator2
      (if true
        ;[1 1 1] Only when the amount of players increases; do something
        (Development|PrintString "Someone Landed on a  Tile")
        (for _array_element (Variables|Default|GetGameComponents)
          (Default|Execute _array_element))))))
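; Game state for a turn-based multiplayer tile board game, tracking match phase, players, money and the current player.
; Placing every player moves the match from Pre Game to In Game, whose authority-side RepNotify shows start text or picks the first turn.
; In-game tile assignments poll until tile effects finish, then ask player controller 0 to pick the next player.
; Name and money updates reach each player's HUD; Tick prints debug state.
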(event Custom|Debug%20State
  ;[1 1 1] TEMP - All for debug
  (if (Pawn|IsLocalController (Game|GetPlayerController 0))
    (Development|PrintString (Utilities|String|EnumtoString (Variables|MatchState|GetCurrent%20Match%20State)) true true "(R=0.000000,G=0.660000,B=1.000000,A=1.000000)" 0.0)))

(event Custom|Server%20Update%20Player%20Names
  ;[1 1 1] Update player Names + Money
  (Utilities|Array|Clear (Variables|Default|GetPlayerNames))
  (for _array_element (Variables|Default|GetPlayerArray)
    (bind _asps_game (Utilities|Casting|CastToPS_Game _array_element))
    (Utilities|Array|Add (Variables|Default|GetPlayerNames) (Variables|/Game/Blueprints/Game/PS_Game.PS_Game_C|GetUserName _asps_game)))
  (for _array_element_2 (Variables|Default|GetPlayerArray)
    (bind _aspc_game (Utilities|Casting|CastToPC_Game (Game|GetPlayerController _array_element_2)))
    (Default|LocalUpdateGameHUD _aspc_game (Variables|Default|GetPlayerNames) (Variables|Default|GetPlayerMoney))))

(event Custom|Server%20Update%20Player%20Money
  ;[1 1 1] Update player Names + Money
  (Utilities|Array|Clear (Variables|Default|GetPlayerMoney))
  (for _array_element (Variables|Default|GetPlayerArray)
    (bind _asps_game (Utilities|Casting|CastToPS_Game _array_element))
    (Utilities|Array|Add (Variables|Default|GetPlayerMoney) (Variables|/Game/Blueprints/Game/PS_Game.PS_Game_C|GetMoney _asps_game)))
  (for _array_element_2 (Variables|Default|GetPlayerArray)
    (bind _aspc_game (Utilities|Casting|CastToPC_Game (Game|GetPlayerController _array_element_2)))
    (Default|LocalUpdateGameHUD _aspc_game (Variables|Default|GetPlayerNames) (Variables|Default|GetPlayerMoney))))

(event Custom|Switch%20Match%20State
  (params (New%20State :type ENUM_MatchState%20Enum :default "NewEnumerator0"))
  (Variables|MatchState|SetCurrent%20Match%20State New%20State))

(event Custom|Assign%20Player%20To%20Tile
  (params (Player :type PC%20Game%20Object%20Reference) (New%20Tile :type BP%20Tile%20Object%20Reference))
  (bind _asps_game (Utilities|Casting|CastToPS_Game (Variables|/Script/Engine.Controller|GetPlayerState Player)))
  (CallFunction|RemovePlayerfromTiles _asps_game)
  (Default|AddPlayer New%20Tile _asps_game)
  (switch Utilities|FlowControl|Switch|SwitchonENUM_MatchState (Variables|MatchState|GetCurrent%20Match%20State)
    (:NewEnumerator1
      (bind _result (Math|Integer|IncrementInt (Variables|Default|GetPlayersPlacedCount))
        (:%20%20
          (if (>= _result (Utilities|Array|Length (Variables|Default|GetPlayerArray)))
            (CallFunction|SwitchMatchState "NewEnumerator2")))))
    (:NewEnumerator2
      ;[1 1 1] Wait for the tile to execute their effects first, if done reset
      (Utilities|Wait (Variables|/Game/Blueprints/Game/Logic/BP_Tile.BP_Tile_C|GetIsDone New%20Tile)
        (:Out
          (Default|ResetIsDone New%20Tile)
          (bind _aspc_game (Utilities|Casting|CastToPC_Game (Game|GetPlayerController 0)))
          (Default|CallPickPlayer _aspc_game))))))

(event Custom|Remove%20Player%20From%20Tiles
  (params (Player :type PS%20Game%20Object%20Reference))
  (for _array_element (Variables|Default|GetTiles)
    (Utilities|Array|RemoveItem (Variables|/Game/Blueprints/Game/Logic/BP_Tile.BP_Tile_C|GetPlayers _array_element) Player)))

(event Custom|Set%20New%20Current%20Player
  (params (Player :type Player%20State%20Object%20Reference))
  (bind _output_get (Variables|Default|SetCurrentPlayer Player))
  (bind _aspc_game (Utilities|Casting|CastToPC_Game (Game|GetPlayerController _output_get))
    (:then
      (Default|DoTurn _aspc_game))
    (:CastFailed
      (Development|PrintString "Set new current player failed. GS_Game"))))

(event EventBeginPlay
  (bind _outactors (Actor|GetAllActorsOfClass "/Game/Blueprints/Game/Logic/BP_Tile.BP_Tile_C"))
  (Variables|Default|SetTiles _outactors))

(event EventTick
  (params (DeltaSeconds :type Float%20%28single-precision%29))
  ;[1 1 1] TEMP - All for debug
  (CallFunction|DebugState))

(fn ConstructionScript)

(fn OnRepCurrentMatchState
  (Networking|SwitchHasAuthority
    (:Authority
      (switch Utilities|FlowControl|Switch|SwitchonENUM_MatchState (Variables|MatchState|GetCurrent%20Match%20State)
        (:NewEnumerator1
          (for _array_element (Variables|Default|GetPlayerArray)
            (bind _aspc_game (Utilities|Casting|CastToPC_Game (Game|GetPlayerController _array_element)))
            (Default|LocalCreateStartText _aspc_game)))
        (:NewEnumerator2
          (bind _player (CallFunction|PickNextPlayer))
          (bind _aspc_game_2 (Utilities|Casting|CastToPC_Game (Game|GetPlayerController 0)))
          (Default|LocalSetNewPlayer _aspc_game_2 _player))))))

(fn FindTileOfPlayer
  (params (Player :type PC%20Game%20Object%20Reference))
  (bind _asps_game (Utilities|Casting|CastToPS_Game (Variables|/Script/Engine.Controller|GetPlayerState Player)))
  (for _array_element (Variables|Default|GetTiles)
    (if (!= (Utilities|Array|FindItem (Variables|/Game/Blueprints/Game/Logic/BP_Tile.BP_Tile_C|GetPlayers _array_element) _asps_game) -1)
      (return _array_element))))

(fn GetNextTile
  (params (Start%20Tile :type BP%20Tile%20Object%20Reference))
  (return (Variables|/Game/Blueprints/Game/Logic/BP_Tile.BP_Tile_C|GetNext%20Tile Start%20Tile)))

(fn PickNextPlayer
  (bind _playerarray (Variables|Default|GetPlayerArray))
  (bind _currentplayer (Variables|Default|GetCurrentPlayer))
  (bind _returnvalue (Utilities|Array|FindItem _playerarray _currentplayer))
  (bind _returnvalue_2 (+ _returnvalue 1))
  (if (or (== (Utilities|Array|Length _playerarray) _returnvalue_2) (== (Variables|Default|GetCurrentPlayer) 0))
    (LocalVariables|SetPickedPlayer (Utilities|Array|Get(acopy) (Variables|Default|GetPlayerArray)))
    (else
      (LocalVariables|SetPickedPlayer (Utilities|Array|Get(acopy) (Variables|Default|GetPlayerArray) _returnvalue_2))))
  (return (LocalVariables|GetPickedPlayer)))
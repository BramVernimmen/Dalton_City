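; Lobby player controller that shows the lobby menu and registers the player's name with the server.
; On local BeginPlay it creates the menu, reads the name from BP_GameInstance client-side, sends it to the server and has GS_Lobby announce the join.
; The PlayerName RepNotify asks GS_Lobby to refresh the name list.
; Local events display a single replaceable join popup and update the menu, recreating it if null.
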(event Custom|UpdatePlayerNames
  (bind _asgs_lobby (Utilities|Casting|CastToGS_Lobby (Game|GetGameState)))
  (Default|ServerUpdatePlayerNames _asgs_lobby))

(event Custom|Local%20Display%20Player%20Joined%20Name
  (params (Player%20Name :type String))
  (Utilities|FlowControl|Sequence
    (:then_0
      ;[1 1 1] if there already is a join message, remove it
      (Utilities|IsValid (Variables|Default|GetJoined%20Player%20Widget)
        (:Is%20Valid
          (Widget|RemovefromParent (Variables|Default|GetJoined%20Player%20Widget)))))
    (:then_1
      (bind _returnvalue (UserInterface|CreateWidget "/Game/Widgets/Lobby_Widgets/WB_JoinedPlayer.WB_JoinedPlayer_C" self (Utilities|Text|ToText(String) Player%20Name)))
      (bind _output_get (Variables|Default|SetJoined%20Player%20Widget _returnvalue))
      (UserInterface|Viewport|AddtoViewport _output_get 0))))

(event Custom|Local%20UpdateLobbyMenu
  (params (PlayerNames :type Array%20of%20Strings))
  (bind _lobbymenu (Variables|Default|GetLobbyMenu))
  (if (== _lobbymenu 0)
    ;[1 1 1] There are times where lobby menu is null, safety recreate it
    (CallFunction|CreateLobbyScreen))
  (Default|SetPlayerNames _lobbymenu PlayerNames))

(event Custom|ServerSetPlayerName
  (params (Player%20Name :type String))
  ;[1 1 1] After getting it locally, set it as the server
  (Variables|Default|SetPlayerName Player%20Name))

(event Custom|InitializeName
  ;[1 1 1] We need to correctly get our Player Name, which is stored in the Game Instance
  (CallFunction|LocalInitializePlayerName))

(event Custom|Local%20Initialize%20Player%20Name
  ;[1 1 1] First get it locally, otherwise you will use the GameInstance of the Server
  (CallFunction|ServerSetPlayerName (CallFunction|GetPlayerName)))

(event Custom|Server%20Display%20Player%20Joined
  (bind _asgs_lobby (Utilities|Casting|CastToGS_Lobby (Game|GetGameState)))
  (Default|DisplayPlayerJoined _asgs_lobby (Variables|Default|GetPlayerName)))

(event EventBeginPlay
  (if (Pawn|IsLocalController)
    (Utilities|FlowControl|Sequence
      (:then_0
        (CallFunction|CreateLobbyScreen))
      (:then_1
        (CallFunction|InitializeName))
      (:then_2
        (CallFunction|ServerDisplayPlayerJoined)))))

(fn ConstructionScript)

(fn GetPlayerName
  (bind _asbp_game_instance (Utilities|Casting|CastToBP_GameInstance (Game|GetGameInstance)))
  (return (Variables|/Game/Blueprints/BP_GameInstance.BP_GameInstance_C|GetPlayerName _asbp_game_instance)))

(fn CreateLobbyScreen
  (bind _returnvalue (UserInterface|CreateWidget "/Game/Widgets/Lobby_Widgets/WB_LobbyMenu.WB_LobbyMenu_C" self))
  (bind _output_get (Variables|Default|SetLobbyMenu _returnvalue))
  (UserInterface|Viewport|AddtoViewport _output_get 0)
  (Variables|Default|SetbShowMouseCursor true))

(fn OnRepPlayerName
  (if (Pawn|IsLocalController)
    (CallFunction|UpdatePlayerNames)))
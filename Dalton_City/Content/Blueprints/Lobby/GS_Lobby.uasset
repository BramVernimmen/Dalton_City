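; Lobby GameState that keeps every player's lobby screen informed about who is present.
; DisplayPlayerJoined loops over PlayerArray and passes the new player's name to each PC_Lobby controller for display.
; ServerUpdatePlayerNames rebuilds the PlayerNames list from those controllers, leaving out PlayerToIgnore, then sends it to the remaining controllers to update their lobby menus.
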(event Custom|Server%20Update%20Player%20Names
  (params (Player%20To%20Ignore :type PC%20Lobby%20Object%20Reference))
  (Utilities|Array|Clear (Variables|Default|GetPlayerNames))
  (for _array_element (Variables|Default|GetPlayerArray)
    (bind _aspc_lobby (Utilities|Casting|CastToPC_Lobby (Game|GetPlayerController _array_element)))
    (if (not (== _aspc_lobby Player%20To%20Ignore))
      (Utilities|Array|Add (Variables|Default|GetPlayerNames) (Variables|/Game/Blueprints/Lobby/PC_Lobby.PC_Lobby_C|GetPlayerName _aspc_lobby))))
  (for _array_element_2 (Variables|Default|GetPlayerArray)
    (bind _aspc_lobby_2 (Utilities|Casting|CastToPC_Lobby (Game|GetPlayerController _array_element_2)))
    (if (not (== _aspc_lobby_2 Player%20To%20Ignore))
      (Default|LocalUpdateLobbyMenu _aspc_lobby_2 (Variables|Default|GetPlayerNames)))))

(event Custom|Display%20Player%20Joined
  (params (PlayerName :type String))
  (for _array_element (Variables|Default|GetPlayerArray)
    (bind _aspc_lobby (Utilities|Casting|CastToPC_Lobby (Game|GetPlayerController _array_element)))
    (Default|LocalDisplayPlayerJoinedName _aspc_lobby PlayerName)))

(fn ConstructionScript)